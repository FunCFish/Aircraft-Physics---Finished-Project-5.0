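; Bullet projectile actor that is fired by an aircraft pawn and removes itself ten seconds after spawning.
; Each tick it casts its owner to BP_AircraftPawn and sets the ProjectileMovement initial and max speeds to the aircraft's scaled Speed plus a base offset.
; Both values keep tracking the owner's current speed after spawn, and velocity is never written directly.
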(event EventTick
  (params (DeltaSeconds :type Float%20%28single-precision%29))
  (bind _projectilemovement (Variables|Default|GetProjectileMovement))
  (bind _asbp_aircraft_pawn (Utilities|Casting|CastToBP_AircraftPawn (Components|GetOwner)))
  (Variables|/Script/Engine.ProjectileMovementComponent|SetInitialSpeed _projectilemovement (+ (* (Variables|/Game/Blueprints/BP_AircraftPawn.BP_AircraftPawn_C|Getspeed _asbp_aircraft_pawn) 1e+05) 1e+04))
  (Variables|/Script/Engine.ProjectileMovementComponent|SetMaxSpeed _projectilemovement (+ (* (Variables|/Game/Blueprints/BP_AircraftPawn.BP_AircraftPawn_C|Getspeed _asbp_aircraft_pawn) 1e+05) 1e+04)))

(event EventBeginPlay
  (Utilities|FlowControl|Delay 1e+01)
  (Actor|DestroyActor))

(fn ConstructionScript)